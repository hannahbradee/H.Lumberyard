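; BP_Enemy_AI is an enemy that chases the player once pawn sensing spots a pawn.
; Sensing sets IsSeeingPlayer and starts an AI MoveTo toward player 0, while Tick halts movement whenever that flag is false.
; The flag effectively latches, as it is only cleared where already false.
; Attacking is a stub: arrival triggers a delay, and CanAttack is never set true.
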(event OnSeePawn(PawnSensing)
  (params (Pawn :type Pawn%20Object%20Reference))
  (Variables|Default|Setis%20Seeing%20Player true)
  (CallFunction|FollowPlayer))

(event Custom|followPlayer
  (Variables|Default|SetcanAttack false)
  (if (Variables|Default|Getis%20Seeing%20Player)
    (AI|AIMoveTo self "0, 0, 0" (Game|GetPlayerCharacter 0) 7e+01 false
      (:OnSuccess
        (if (not (Variables|Default|GetcanAttack))
          (Variables|Default|SetcanAttack false)
          ;[1 1 1] add attack animation before delay and set to can attack
          (Utilities|FlowControl|Delay 1.0)
          (Variables|Default|SetcanAttack false))))
    (else
      (Variables|Default|Setis%20Seeing%20Player false))))

(event EventBeginPlay)

(event Collision|EventActorBeginOverlap
  (params (OtherActor :type Actor%20Object%20Reference)))

(event EventTick
  (params (DeltaSeconds :type Float%20%28single-precision%29))
  (if (not (Variables|Default|Getis%20Seeing%20Player))
    (Components|Movement|StopMovementImmediately (Variables|Character|GetCharacterMovement))))

(fn ConstructionScript)